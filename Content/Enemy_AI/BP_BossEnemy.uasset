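; Boss enemy character with a greatsword, six melee attacks, a lightning strike, a teleport and a health bar widget updated on damage.
; Montage notifies spawn or destroy the sword and trigger forward sphere traces that damage Player-tagged pawns.
; Lightning spawns an AOE actor, then sphere-traces it after a delay.
; Teleport is a hidden, high-speed AI flight with a particle trail; dispatchers signal when actions end.
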(event Custom|Attack1
  (params (Attack%20Target :type Actor%20Object%20Reference))
  (Variables|Default|SetDamage 5.0)
  (bind _notifyname (Animation|Montage|PlayMontage (Variables|Character|GetMesh) "/Game/Enemy_AI/AI/Animations/Greatsword/Attacks/Montages/GreatSwordSlashLong_UE_Montage.GreatSwordSlashLong_UE_Montage")
    (:OnCompleted
      (Default|CallOnAttackEnd :!label _label))
    (:OnInterrupted
      (goto _label))
    (:OnNotifyBegin
      (switch name _notifyname
        (:Slash
          (CallFunction|AttackDamage 4e+01 2.2e+02))))))

(event Custom|Lightning%20Strike
  (params (Attack%20Target :type Actor%20Object%20Reference))
  (bind _notifyname (Animation|Montage|PlayMontage (Variables|Character|GetMesh) "/Game/Enemy_AI/AI/Animations/Greatsword/Attacks/Montages/GreatSwordCasting_UE_Montage.GreatSwordCasting_UE_Montage")
    (:OnCompleted
      (Default|CallOnAttackEnd :!label _label))
    (:OnInterrupted
      (goto _label))
    (:OnNotifyBegin
      (switch name _notifyname
        (:Lightning
          (bind _returnvalue (Game|SpawnActorfromClass "/Game/Enemy_AI/AOE/AOE_Lightning.AOE_Lightning_C" (Math|Transform|MakeTransform "0, 0, 0" "0, 0, 0" "1.000000,1.000000,1.000000") "Undefined" "MultiplyWithRoot" 0 1.0 Attack%20Target 0))
          (Utilities|FlowControl|Delay 1.3)
          (bind (_outhit _returnvalue_2) (Collision|SphereTraceForObjects (Transformation|GetActorLocation _returnvalue) (Transformation|GetActorLocation _returnvalue) 1.5e+02 (Utilities|Array|MakeArray "ObjectTypeQuery3") false 0 "ForDuration"))
          (if _returnvalue_2
            (if (Actor|ActorHasTag (.HitActor (Collision|BreakHitResult _outhit)) "Player")
              (Utilities|FlowControl|DoOnce false :!label _label_2
                (:Completed
                  (Game|Damage|ApplyDamage (.HitActor (Collision|BreakHitResult _outhit)) 3.0 0 0)
                  (Utilities|FlowControl|Delay 0.2)
                  (goto _label_2 Reset))))))))))

(event Custom|Teleport
  (params (Location :type Vector) (Attack%20Target :type Actor%20Object%20Reference))
  (bind _charactermovement (Variables|Character|GetCharacterMovement))
  (bind _mesh (Variables|Character|GetMesh))
  ;[1 1 1] teleport
  (if (not (Variables|Default|GetIsTeleporting))
    (Variables|Default|SetIsTeleporting true)
    (Pawn|Components|CharacterMovement|SetMovementMode _charactermovement "MOVE_Flying" 0)
    (Variables|/Script/Engine.CharacterMovementComponent|SetMaxFlySpeed _charactermovement 5e+03)
    (Variables|/Script/Engine.CharacterMovementComponent|SetMaxAcceleration _charactermovement 999999.0)
    (Rendering|SetVisibility _mesh false true)
    (Collision|SetCollisionResponsetoChannel (Variables|Default|GetCapsuleComponent) "ECC_Pawn" "ECR_Ignore")
    (bind _returnvalue (Effects|SpawnEmitterAttached 0 _mesh "spine_01"))
    (Variables|Default|SetTeleportTrailEffect _returnvalue)
    (Animation|StopAnimMontage 0)
    (AI|AIMoveTo self Location Attack%20Target 1.5e+02 false
      (:OnSuccess
        _)
      (:OnFail
        _))
    (CallFunction|TeleportEnd)
    (else
      (Utilities|FlowControl|DelayUntilNextTick)
      (Default|CallOnTeleportEnd))))

(event Custom|Teleport%20End
  (bind _charactermovement (Variables|Character|GetCharacterMovement))
  ;[1 1 1] teleport
  (Components|Movement|StopMovementImmediately _charactermovement)
  (Pawn|Components|CharacterMovement|SetMovementMode _charactermovement "MOVE_Walking" 0)
  (Variables|/Script/Engine.CharacterMovementComponent|SetMaxAcceleration _charactermovement 1.5e+03)
  (Rendering|SetVisibility (Variables|Character|GetMesh) true true)
  (Collision|SetCollisionResponsetoChannel (Variables|Default|GetCapsuleComponent) "ECC_Pawn" "ECR_Block")
  (Default|CallOnTeleportEnd)
  (Utilities|FlowControl|Delay 0.5)
  (Variables|Default|SetIsTeleporting false)
  (bind _teleporttraileffect (Variables|Default|GetTeleportTrailEffect)
    (:then
      (Components|DestroyComponent _teleporttraileffect))
    (:else)))

(event Custom|Attack6
  (params (Attack%20Target :type Actor%20Object%20Reference))
  (Variables|Default|SetDamage 5.0)
  (bind _notifyname (Animation|Montage|PlayMontage (Variables|Character|GetMesh) "/Game/Enemy_AI/AI/Animations/Greatsword/Attacks/Montages/GreatSwordKick2_UE_Montage.GreatSwordKick2_UE_Montage")
    (:OnCompleted
      (Default|CallOnAttackEnd :!label _label))
    (:OnInterrupted
      (goto _label))
    (:OnNotifyBegin
      (switch name _notifyname
        (:Kick
          (CallFunction|AttackDamage 4e+01 1e+02))))))

(event Custom|Attack%20Damage
  (params (Radius :type Float%20%28double-precision%29) (Length :type Float%20%28double-precision%29))
  (bind _returnvalue (Transformation|GetActorLocation))
  ;[1 1 1] Hit Detection and Damage
  (bind (_outhit _returnvalue_2) (Collision|SphereTraceForObjects _returnvalue (+ _returnvalue (* (Transformation|GetActorForwardVector (Components|GetOwner)) Length)) Radius (Utilities|Array|MakeArray "ObjectTypeQuery3") false 0 "ForDuration"))
  (if _returnvalue_2
    (if (Actor|ActorHasTag (.HitActor (Collision|BreakHitResult _outhit)) "Player")
      (Utilities|FlowControl|DoOnce false :!label _label
        (:Completed
          (Game|Damage|ApplyDamage (.HitActor (Collision|BreakHitResult _outhit)) (Variables|Default|GetDamage) 0 0)
          (Utilities|FlowControl|Delay 0.2)
          (goto _label Reset))))))

(event Custom|OnAOEOverlapActor_Event
  (params (Actor :type Actor%20Object%20Reference))
  (if (Actor|ActorHasTag (.HitActor (Collision|BreakHitResult (stale Custom|Lightning%20Strike _outhit))) "Player")
    (Utilities|FlowControl|DoOnce false :!label _label
      (:Completed
        (Game|Damage|ApplyDamage (.HitActor (Collision|BreakHitResult (stale Custom|Lightning%20Strike _outhit))) 3.0 0 0)
        (Utilities|FlowControl|Delay 0.2)
        (goto _label Reset)))))

(event Custom|Attack2
  (params (Attack%20Target :type Actor%20Object%20Reference))
  (Variables|Default|SetDamage 5.0)
  (bind _notifyname (Animation|Montage|PlayMontage (Variables|Character|GetMesh) "/Game/Enemy_AI/AI/Animations/Greatsword/Attacks/Montages/GreatSwordHighSpinAttack_UE_Montage.GreatSwordHighSpinAttack_UE_Montage")
    (:OnCompleted
      (Default|CallOnAttackEnd :!label _label))
    (:OnInterrupted
      (goto _label))
    (:OnNotifyBegin
      (switch name _notifyname
        (:Slash
          (CallFunction|AttackDamage 4e+01 2.2e+02))))))

(event Custom|Attack3
  (params (Attack%20Target :type Actor%20Object%20Reference))
  (Variables|Default|SetDamage 2.0)
  (bind _notifyname (Animation|Montage|PlayMontage (Variables|Character|GetMesh) "/Game/Enemy_AI/AI/Animations/Greatsword/Attacks/Montages/GreatSwordKick_UE_Montage.GreatSwordKick_UE_Montage")
    (:OnCompleted
      (Default|CallOnAttackEnd :!label _label))
    (:OnInterrupted
      (goto _label))
    (:OnNotifyBegin
      (switch name _notifyname
        (:Kick
          (CallFunction|AttackDamage 4e+01 1e+02))))))

(event Custom|Attack4
  (params (Attack%20Target :type Actor%20Object%20Reference))
  (Variables|Default|SetDamage 5.0)
  (bind _notifyname (Animation|Montage|PlayMontage (Variables|Character|GetMesh) "/Game/Enemy_AI/AI/Animations/Greatsword/Attacks/Montages/GreatSwordSlash_1__UE_Montage.GreatSwordSlash_1__UE_Montage")
    (:OnCompleted
      (Default|CallOnAttackEnd :!label _label))
    (:OnInterrupted
      (goto _label))
    (:OnNotifyBegin
      (switch name _notifyname
        (:Slash
          (CallFunction|AttackDamage 4e+01 2.2e+02))))))

(event Custom|Attack5
  (params (Attack%20Target :type Actor%20Object%20Reference))
  (Variables|Default|SetDamage 5.0)
  (bind _notifyname (Animation|Montage|PlayMontage (Variables|Character|GetMesh) "/Game/Enemy_AI/AI/Animations/Greatsword/Attacks/Montages/GreatSwordSlash_2__UE_Montage.GreatSwordSlash_2__UE_Montage")
    (:OnCompleted
      (Default|CallOnAttackEnd :!label _label))
    (:OnInterrupted
      (goto _label))
    (:OnNotifyBegin
      (switch name _notifyname
        (:Slash
          (CallFunction|AttackDamage 4e+01 2.2e+02))))))

(event EventBeginPlay
  (Variables|Default|SetCurrent%20Health (Variables|Default|GetMax%20Health))
  (bind _returnvalue (UserInterface|CreateWidget "/Game/UI/Boss_HealthBar.Boss_HealthBar_C"))
  (bind _output_get (Variables|Default|SetBoss%20Health%20Bar%20Ref _returnvalue))
  (Default|UpdateHeath _output_get (Variables|Default|GetCurrent%20Health) (Variables|Default|GetMax%20Health)))

(event Collision|EventActorBeginOverlap
  (params (OtherActor :type Actor%20Object%20Reference)))

(event EventTick
  (params (DeltaSeconds :type Float%20%28single-precision%29)))

(event EventEquipSword
  (bind _notifyname (Animation|Montage|PlayMontage (Variables|Character|GetMesh) "/Game/Enemy_AI/AI/Animations/Greatsword/Equip_and_Unequip/Montages/DrawAGreatSword2_UE_Montage.DrawAGreatSword2_UE_Montage")
    (:OnCompleted
      (Default|CallOnSwordDraw))
    (:OnNotifyBegin
      (switch name _notifyname
        (:Sword%20Draw
          (bind _returnvalue (Game|SpawnActorfromClass "/Game/Enemy_AI/Weapons/BP_Greatsword.BP_Greatsword_C" (Transformation|GetActorTransform) "Undefined" "MultiplyWithRoot" 0 0))
          (bind _output_get (Variables|Default|SetSword%20Actor _returnvalue))
          (Transformation|AttachComponentToComponent _output_get (Variables|Character|GetMesh) "Weapon" "SnapToTarget" "SnapToTarget" "SnapToTarget" true)
          (Variables|Default|SetIsWieldingWeapon true))))))

(event EventUnequipSword
  (bind _notifyname (Animation|Montage|PlayMontage (Variables|Character|GetMesh) "/Game/Enemy_AI/AI/Animations/Greatsword/Equip_and_Unequip/Montages/SheathAGreatSword1_UE_Montage.SheathAGreatSword1_UE_Montage")
    (:OnCompleted
      (Default|CallOnSwordSheath))
    (:OnNotifyBegin
      (switch name _notifyname
        (:Sheath%20Sword
          (Actor|DestroyActor (Variables|Default|GetSword%20Actor))
          (Variables|Default|SetIsWieldingWeapon false))))))

(event Game|Damage|EventAnyDamage
  (params (Damage :type Float%20%28single-precision%29) (DamageType :type Damage%20Type%20Object%20Reference) (InstigatedBy :type Controller%20Object%20Reference) (DamageCauser :type Actor%20Object%20Reference))
  (bind _output_get (Variables|Default|SetCurrent%20Health (- (Variables|Default|GetCurrent%20Health) Damage)))
  (Default|UpdateHeath (Variables|Default|GetBoss%20Health%20Bar%20Ref) _output_get (Variables|Default|GetMax%20Health)))

(fn ConstructionScript
  (|CallParentFunction))

(fn SetMovementSpeed
  (params (Speed :type E_MoveSpeed%20Enum :default "NewEnumerator0"))
  (bind _output_get (Variables|/Script/Engine.CharacterMovementComponent|SetMaxWalkSpeed (Variables|Character|GetCharacterMovement) (Utilities|Select :Index Speed :NewEnumerator0 0.0 :NewEnumerator1 1e+02 :NewEnumerator2 2e+02 :NewEnumerator3 3.5e+02)))
  (return _output_get))