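; BP_BossSpawner is an actor that spawns the boss enemy at its location and respawns it on reset.
; BeginPlay and ResetBoss both call SpawnEnemy, which destroys any existing boss and a BP_Greatsword found in the level, then spawns and stores a new BP_BossEnemy.
; The skeletal mesh supplies the spawn rotation.
; Leftover logic checking whether the boss is dead is disconnected and never runs.
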(event Custom|Spawn%20Enemy
  (Utilities|IsValid (Variables|Default|GetSpawned%20Boss)
    (:Is%20Valid
      (Actor|DestroyActor (Variables|Default|GetSpawned%20Boss))
      (bind _returnvalue (Actor|GetActorOfClass "/Game/Enemy_AI/Weapons/BP_Greatsword.BP_Greatsword_C"))
      (Utilities|IsValid _returnvalue
        (:Is%20Valid
          (Actor|DestroyActor _returnvalue))
        (:Is%20Not%20Valid
          _)))
    (:Is%20Not%20Valid
      _))
  (bind _returnvalue_2 (Game|SpawnActorfromClass "/Game/Enemy_AI/BP_BossEnemy.BP_BossEnemy_C" (Math|Transform|MakeTransform (Transformation|GetActorLocation) (Transformation|GetWorldRotation (Variables|Default|GetSkeletalMesh)) "1.000000,1.000000,1.000000") "AlwaysSpawn" "MultiplyWithRoot" 0 0))
  (Variables|Default|SetSpawned%20Boss _returnvalue_2))

(event EventBeginPlay
  (CallFunction|SpawnEnemy))

(event EventResetBoss
  (CallFunction|SpawnEnemy))

(fn ConstructionScript)