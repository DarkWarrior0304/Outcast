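; Melee enemy that draws, swings and sheathes a greatsword, with a floating health bar above it.
; Attack, equip and unequip events play montages and fire end dispatchers so the caller knows when each action finishes.
; Montage notifies time spawning the sword onto the Weapon socket and destroying it, toggling the wielding flag.
; Tick turns the health bar toward the player camera and refreshes its fill from current health.
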(event Custom|Sheath%20Swords)

(event Custom|Attacks)

(event Custom|Wield%20Sword)

(event EventEquipSword
  (bind _notifyname (Animation|Montage|PlayMontage (Variables|Character|GetMesh) "/Game/Enemy_AI/AI/Animations/Greatsword/Equip_and_Unequip/Montages/DrawAGreatSword2_UE_Montage.DrawAGreatSword2_UE_Montage")
    (:OnCompleted
      (Default|CallOnSwordDraw))
    (:OnNotifyBegin
      (switch name _notifyname
        (:Sword%20Draw
          (bind _returnvalue (Game|SpawnActorfromClass "/Game/Enemy_AI/Weapons/BP_Greatsword.BP_Greatsword_C" (Transformation|GetActorTransform) "Undefined" "MultiplyWithRoot" 0 0))
          (bind _output_get (Variables|Default|SetSword%20Actor _returnvalue))
          (Transformation|AttachComponentToComponent _output_get (Variables|Character|GetMesh) "Weapon" "SnapToTarget" "SnapToTarget" "SnapToTarget" true)
          (Variables|Default|SetIsWieldingWeapon true))))))

(event EventUnequipSword
  (bind _notifyname (Animation|Montage|PlayMontage (Variables|Character|GetMesh) "/Game/Enemy_AI/AI/Animations/Greatsword/Equip_and_Unequip/Montages/SheathAGreatSword1_UE_Montage.SheathAGreatSword1_UE_Montage")
    (:OnCompleted
      (Default|CallOnSwordSheath))
    (:OnNotifyBegin
      (switch name _notifyname
        (:Sheath%20Sword
          (Actor|DestroyActor (Variables|Default|GetSword%20Actor))
          (Variables|Default|SetIsWieldingWeapon false))))))

(event EventAttack
  (Animation|Montage|PlayMontage (Variables|Character|GetMesh) "/Game/Enemy_AI/AI/Animations/Greatsword/Attacks/Montages/GreatSwordSlash_UE_Montage.GreatSwordSlash_UE_Montage"
    (:OnCompleted
      _)
    (:OnInterrupted
      _))
  (Default|CallOnAttackEnd))

(event EventBeginPlay
  (Utilities|FlowControl|Sequence
    (:then_0
      (Utilities|Casting|CastToEnemy_Health (UserInterface|GetWidget (Variables|Default|GetHealthBar))))
    (:then_1
      (Variables|Default|SetCurrent%20Health (Variables|Default|GetMax%20Health)))))

(event EventTick
  (params (DeltaSeconds :type Float%20%28single-precision%29))
  (Utilities|FlowControl|Sequence
    (:then_0
      (Transformation|SetWorldRotation (Variables|Default|GetHealthBar) (Math|Rotator|FindLookatRotation (Transformation|GetWorldLocation (Variables|Default|GetHealthBar)) (Transformation|GetWorldLocation (Variables|/Script/Engine.PlayerCameraManager|GetTransformComponent (Game|GetPlayerCameraManager 0)))) false false))
    (:then_1
      (CallFunction|UpdateHealthBar))))

(fn ConstructionScript
  (|CallParentFunction))

(fn UpdateHealthBar
  (bind _asenemy_health (Utilities|Casting|CastToEnemy_Health (UserInterface|GetWidget (Variables|Default|GetHealthBar))))
  (Progress|SetPercent (Variables|/Game/UI/Enemy_Health.Enemy_Health_C|GetHealthBar _asenemy_health) (/ (Variables|Default|GetCurrent%20Health) (Variables|Default|GetMax%20Health)))
  (return))