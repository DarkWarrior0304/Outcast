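; Enemy spawner actor that creates a BP_MeleeEnemy at its location on BeginPlay and respawns it when ResetEnemies is called.
; The spawn takes its rotation from the spawner's skeletal mesh and passes the PatrolRoute to the new enemy.
; Before respawning, it destroys the tracked enemy if still valid, along with the first BP_Sword found in the level, which is not necessarily that enemy's.
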(event Custom|Spawn%20Enemy
  (Utilities|IsValid (Variables|Default|GetSpawned%20Enemy)
    (:Is%20Valid
      (Actor|DestroyActor (Variables|Default|GetSpawned%20Enemy))
      (bind _returnvalue (Actor|GetActorOfClass "/Game/Enemy_AI/Weapons/BP_Sword.BP_Sword_C"))
      (Utilities|IsValid _returnvalue
        (:Is%20Valid
          (Actor|DestroyActor _returnvalue))
        (:Is%20Not%20Valid
          _)))
    (:Is%20Not%20Valid
      _))
  (bind _returnvalue_2 (Game|SpawnActorfromClass "/Game/Enemy_AI/BP_MeleeEnemy.BP_MeleeEnemy_C" (Math|Transform|MakeTransform (Transformation|GetActorLocation) (Transformation|GetWorldRotation (Variables|Default|GetSkeletalMesh)) "1.000000,1.000000,1.000000") "AlwaysSpawn" "MultiplyWithRoot" 0 (Variables|Default|GetPatrol%20Route) 0))
  (Variables|Default|SetSpawned%20Enemy _returnvalue_2))

(event EventBeginPlay
  (CallFunction|SpawnEnemy))

(event EventResetEnemies
  (CallFunction|SpawnEnemy))

(fn ConstructionScript)