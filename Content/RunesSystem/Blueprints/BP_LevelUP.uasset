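; BP_LevelUP is a trigger actor that grants experience when an actor overlaps its box.
; On overlap it checks the player's stats component, proceeding only if ExtractExtraSpiritsFromAttributes returns zero and the component's widget is not visible.
; It then sends EXPToGive to the overlapping actor through ReceiveExperienceMessage, without checking that this actor is the player.
; A DoOnce reset after a one-second delay throttles repeated grants.
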(event OnComponentBeginOverlap(Box)
  (params (OverlappedComponent :type Primitive%20Component%20Object%20Reference) (OtherActor :type Actor%20Object%20Reference) (OtherComp :type Primitive%20Component%20Object%20Reference) (OtherBodyIndex :type Integer) (bFromSweep :type Boolean) (SweepResult :type Hit%20Result%20Structure%20%28by%20ref%29))
  (bind _playercharacter (CallFunction|GetPlayerCharacter))
  (bind _bp_statscomponent (Variables|/Game/RunesSystem/Blueprints/BP_RuneCharacter.BP_RuneCharacter_C|GetBP_StatsComponent _playercharacter))
  (if (and (== (Default|ExtractExtraSpiritsfromAttributes _bp_statscomponent) 0) (not (Variables|/Game/RunesSystem/Blueprints/BP_StatsComponent.BP_StatsComponent_C|GetWidgetVisible? _bp_statscomponent)))
    (Utilities|FlowControl|DoOnce false :!label _label
      (:Completed
        (Class|BPBPIRuneSystem|ReceiveExperience(Message) OtherActor (Variables|Default|GetEXP%20to%20Give))
        (Utilities|FlowControl|Delay 1.0)
        (goto _label Reset)))))

(event EventBeginPlay)

(event Collision|EventActorBeginOverlap
  (params (OtherActor :type Actor%20Object%20Reference)))

(event EventTick
  (params (DeltaSeconds :type Float%20%28single-precision%29)))

(fn ConstructionScript)