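; Player character for the rune system, holding level, experience and gold, and delegating to rune and stats components.
; Experience gains loop through level-ups, raising the requirement, updating stats and unlocking rune slots.
; Events forward rune purchases, swaps, shop toggling, attribute spending and rune stat changes to those components.
; Keys toggle the stats widget with cursor mode, line-trace for NPC interaction, and export textures to a hardcoded local path.
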(fn ConstructionScript)

(fn MouseInput
  (bind _returnvalue (Game|GetPlayerController 0))
  (bind _returnvalue_2 (Game|GetPlayerController 0))
  (if (Variables|Default|GetMouseVisibility?)
    (Variables|/Script/Engine.PlayerController|SetbShowMouseCursor _returnvalue false)
    (Input|SetInputModeGameOnly _returnvalue false)
    (Variables|Default|SetMouseVisibility? false)
    (else
      (Variables|/Script/Engine.PlayerController|SetbShowMouseCursor _returnvalue_2 true)
      (Input|SetInputModeGameandUI _returnvalue_2 0 "DoNotLock" true false)
      (Variables|Default|SetMouseVisibility? true))))

(fn ToggleMoveInput
  (params (bNewMoveInput :type Boolean))
  (Input|SetIgnoreMoveInput (Pawn|GetController) (not bNewMoveInput)))

(event EventToggleMouseInput
  ;[0 0 0] Toggle Mouse Input and Handle Shop Widget Visibility
  (CallFunction|MouseInput))

(event EventToggleMoveIqnoreInput
  (params (CanMove? :type Boolean))
  ;[0 0 0] Toggle Move Input
  (CallFunction|ToggleMoveInput CanMove?))

(event EventChangeStats
  (params (Stats :type Array%20of%20ST%20Stats%20Structures) (Subtract? :type Boolean))
  ;[0 0 0] Modify the stats based on the stats of every rune and update the widget
  (for _array_element Stats
    (Default|ModifyStat (Variables|Default|GetBP_StatsComponent) (.Stat (Utilities|Struct|BreakST_Stats _array_element)) (* (select Subtract? 1.0 -1.0) (.Value (Utilities|Struct|BreakST_Stats _array_element))) 0.0 true (not Subtract?) true))
  (Default|UpdateWidgets (Variables|Default|GetBP_StatsComponent)))

(event EventExperience
  (params (Amount :type Integer))
  (bind _bp_runecomponent (Variables|Default|GetBP_RuneComponent))
  (bind _level (Variables|Default|GetLevel))
  (bind _returnvalue (- _level 1))
  (bind _mainwidget (Default|GetMainWidget _bp_runecomponent))
  (bind _allslots (Default|GetAllRuneSlots _mainwidget))
  (bind _output (Utilities|Array|Get(acopy) _allslots _returnvalue))
  ;[0 0 0] Receive experience and Increase level
  (bind _output_get (Variables|Default|SetCurrentExp (+ Amount (Variables|Default|GetCurrentExp))))
  (while (>= _output_get (Variables|Default|GetNeededExp))
    (Utilities|FlowControl|Sequence
      (:then_0
        (Variables|Default|SetCurrentExp (- (Variables|Default|GetCurrentExp) (Variables|Default|GetNeededExp)))
        (Variables|Default|SetNeededExp (Math|Float|Truncate (* (Variables|Default|GetNeededExp) 1.1)))
        (Math|Integer|IncrementInt (Variables|Default|GetLevel)
          (:%20%20
            (Default|StatsPerLevel (Variables|Default|GetBP_StatsComponent))
            (Default|SaveRuneSlots (Variables|Default|GetBP_RuneComponent))
            (Utilities|IsValid _output
              (:Is%20Valid
                (Default|UnlockRuneSlot _output))))))
      (:then_1
        (Utilities|FlowControl|DoOnce false
          (:Completed
            (Audio|PlaySound2D (Variables|Default|GetLevelUpSound) 1.0 1.0 0.0 0 0))))))
  (Utilities|FlowControl|Delay 1.0)
  (Utilities|FlowControl|DoOnce false) ; enters at Reset
)

(event EventToggleShopWidgetVisibility
  (params (RunesToSell :type Array%20of%20Names))
  ;[0 0 0] Toggle Mouse Input and Handle Shop Widget Visibility
  (Default|ToggleShopVisibility (Variables|Default|GetBP_RuneComponent) RunesToSell))

(event EventUnlockRune
  (params (Rune :type ST%20Rune%20Structure))
  (bind (_sellable_ _sellvalue) (Utilities|Struct|BreakST_Rune Rune))
  ;[0 0 0] Unlock rune if there is enough gold. Subtract the gold after the rune has been unlocked
  (if (and _sellable_ (>= (Variables|Default|GetGold) _sellvalue))
    (Default|UnlockRune (Variables|Default|GetBP_RuneComponent) Rune)
    (Variables|Default|SetGold (- (Variables|Default|GetGold) (Utilities|Struct|BreakST_Rune Rune)))
    (Utilities|Array|Add (Variables|/Game/RunesSystem/Blueprints/BP_RuneComponent.BP_RuneComponent_C|GetLocalRunesBought (Variables|Default|GetBP_RuneComponent)) Rune)))

(event EventSwapRunes
  (params (RuneSlotWidget :type WBP%20Rune%20Slot%20Object%20Reference) (RuneWidget :type WBP%20Rune%20Object%20Reference) (DroppedInRuneWidget? :type Boolean))
  ;[0 0 0] Swap and Move Runes
  (Default|SwapRunes (Variables|Default|GetBP_RuneComponent) RuneSlotWidget RuneWidget DroppedInRuneWidget?))

(event EventMoveRune
  (params (RuneSlotWidget :type WBP%20Rune%20Slot%20Object%20Reference) (RuneWidget :type WBP%20Rune%20Object%20Reference) (DroppedInRuneWidget? :type Boolean))
  ;[0 0 0] Swap and Move Runes
  (Default|MoveRune (Variables|Default|GetBP_RuneComponent) RuneSlotWidget RuneWidget DroppedInRuneWidget?))

(event EventSpendAttributePoints
  (params (Attribute :type ST%20Attributes%20Structure) (Pts :type Integer))
  ;[0 0 0] Spend Attribute Points
  (Default|SpendAttributePoints (Variables|Default|GetBP_StatsComponent) Attribute Pts))

(event Input|KeyboardEvents|2
  (params (Key :type Key%20Structure :default "None"))
  (bind _bp_statscomponent (Variables|Default|GetBP_StatsComponent))
  ;[0 0 0] Handle UI Visibility along with mouse input and input mode
  (:Pressed
    (Default|ToggleStatsWidget _bp_statscomponent)
    (if (Variables|/Game/RunesSystem/Blueprints/BP_StatsComponent.BP_StatsComponent_C|GetWidgetVisible? _bp_statscomponent)
      (if (not (Variables|Default|GetMouseVisibility?))
        (CallFunction|MouseInput :!label _label))
      (elif (not (Variables|/Game/RunesSystem/Blueprints/BP_RuneComponent.BP_RuneComponent_C|GetWidgetVisible? (Variables|Default|GetBP_RuneComponent)))
        (goto _label)))))

(event Input|KeyboardEvents|Z
  (params (Key :type Key%20Structure :default "None"))
  (:Pressed
    (for _array_element (Variables|Default|GetTextures)
      (Class|KismetRenderingLibrary|ExportTexture2D _array_element "C:\\Users\\Billo\\Downloads\\Anthi" (Utilities|String|Append (Utilities|GetObjectName _array_element) ".png")))))

(event Input|KeyboardEvents|E
  (params (Key :type Key%20Structure :default "None"))
  (bind _returnvalue (Transformation|GetActorLocation))
  ;[0 0 0] Handle Interaction with NPC
  (:Pressed
    (bind (_outhit _returnvalue_2) (Collision|LineTraceForObjects _returnvalue (+ _returnvalue (* (Math|Vector|GetForwardVector (Variables|Collision|GetCapsuleComponent)) 150)) (Utilities|Array|MakeArray "ObjectTypeQuery2" "ObjectTypeQuery3") false 0 "ForDuration"))
    (if _returnvalue_2
      (Class|BPBPIInteractable|OnInteract(Message) (.HitActor (Collision|BreakHitResult _outhit)) self))))

(event Input|KeyboardEvents|1
  (params (Key :type Key%20Structure :default "None"))
  ;[0 0 0] Handle UI Visibility along with mouse input and input mode
)

(fn GetCurrentExp
  (return (Variables|Default|GetCurrentExp)))

(fn GetGold
  (return (Variables|Default|GetGold)))

(fn GetMainWidget
  (return (Default|GetMainWidget (Variables|Default|GetBP_RuneComponent))))

(fn GetNeededExp
  (return (Variables|Default|GetNeededExp)))

(fn GetPlayerLevel
  (return (Variables|Default|GetLevel)))

(fn GetRequiredSpirits
  (return (Variables|/Game/RunesSystem/Blueprints/BP_StatsComponent.BP_StatsComponent_C|GetRequiredSpirits (Variables|Default|GetBP_StatsComponent))))

(fn GetSpirits
  (return (Variables|/Game/RunesSystem/Blueprints/BP_StatsComponent.BP_StatsComponent_C|GetSpirits (Variables|Default|GetBP_StatsComponent))))

(fn GetStats
  (return (Variables|/Game/RunesSystem/Blueprints/BP_StatsComponent.BP_StatsComponent_C|GetStats (Variables|Default|GetBP_StatsComponent))))