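; Attacks Blueprint that plays the player character's light and heavy melee combo montages.
; On BeginPlay it caches the player as BP_ThirdPersonCharacter1, whose chain counters track each combo's position.
; Each attack event plays the montage at the current index, then advances the counter through a hard-coded switch that wraps to zero.
; It sets LastAttack on the character when the index reaches the array's final montage.
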(event Custom|HeavyAttack
  (bind _characterref (Variables|Default|GetCharacterRef))
  (bind _characterref_2 (Variables|Default|GetCharacterRef))
  (if (== (+ (Variables|/Game/ThirdPerson/Blueprints/BP_ThirdPersonCharacter1.BP_ThirdPersonCharacter1_C|GetChainHeavyAttack (Variables|Default|GetCharacterRef)) 1) (Utilities|Array|Length (Variables|Default|GetHeavyAttacks)))
    (Variables|/Game/ThirdPerson/Blueprints/BP_ThirdPersonCharacter1.BP_ThirdPersonCharacter1_C|SetLastAttack _characterref true))
  (switch int (Variables|/Game/ThirdPerson/Blueprints/BP_ThirdPersonCharacter1.BP_ThirdPersonCharacter1_C|GetChainHeavyAttack _characterref)
    (:0
      (Animation|PlayAnimMontage _characterref_2 (Utilities|Array|Get(acopy) (Variables|Default|GetHeavyAttacks) (Variables|/Game/ThirdPerson/Blueprints/BP_ThirdPersonCharacter1.BP_ThirdPersonCharacter1_C|GetChainHeavyAttack _characterref_2)) 1.0 "None")
      (Variables|/Game/ThirdPerson/Blueprints/BP_ThirdPersonCharacter1.BP_ThirdPersonCharacter1_C|SetChainHeavyAttack (Variables|Default|GetCharacterRef) 1))
    (:1
      (Animation|PlayAnimMontage _characterref_2 (Utilities|Array|Get(acopy) (Variables|Default|GetHeavyAttacks) (Variables|/Game/ThirdPerson/Blueprints/BP_ThirdPersonCharacter1.BP_ThirdPersonCharacter1_C|GetChainHeavyAttack _characterref_2)) 1.0 "None")
      (Variables|/Game/ThirdPerson/Blueprints/BP_ThirdPersonCharacter1.BP_ThirdPersonCharacter1_C|SetChainHeavyAttack (Variables|Default|GetCharacterRef) 0))))

(event Custom|LightAttack
  (bind _characterref (Variables|Default|GetCharacterRef))
  (bind _characterref_2 (Variables|Default|GetCharacterRef))
  (if (== (+ (Variables|/Game/ThirdPerson/Blueprints/BP_ThirdPersonCharacter1.BP_ThirdPersonCharacter1_C|GetChainLightAttack (Variables|Default|GetCharacterRef)) 1) (Utilities|Array|Length (Variables|Default|GetLightAttacks)))
    (Variables|/Game/ThirdPerson/Blueprints/BP_ThirdPersonCharacter1.BP_ThirdPersonCharacter1_C|SetLastAttack _characterref true))
  (switch int (Variables|/Game/ThirdPerson/Blueprints/BP_ThirdPersonCharacter1.BP_ThirdPersonCharacter1_C|GetChainLightAttack _characterref)
    (:0
      (Animation|PlayAnimMontage _characterref_2 (Utilities|Array|Get(acopy) (Variables|Default|GetLightAttacks) (Variables|/Game/ThirdPerson/Blueprints/BP_ThirdPersonCharacter1.BP_ThirdPersonCharacter1_C|GetChainLightAttack _characterref_2)) 1.0 "None")
      (Variables|/Game/ThirdPerson/Blueprints/BP_ThirdPersonCharacter1.BP_ThirdPersonCharacter1_C|SetChainLightAttack (Variables|Default|GetCharacterRef) 1))
    (:1
      (Animation|PlayAnimMontage _characterref_2 (Utilities|Array|Get(acopy) (Variables|Default|GetLightAttacks) (Variables|/Game/ThirdPerson/Blueprints/BP_ThirdPersonCharacter1.BP_ThirdPersonCharacter1_C|GetChainLightAttack _characterref_2)) 1.0 "None")
      (Variables|/Game/ThirdPerson/Blueprints/BP_ThirdPersonCharacter1.BP_ThirdPersonCharacter1_C|SetChainLightAttack (Variables|Default|GetCharacterRef) 2))
    (:2
      (Animation|PlayAnimMontage _characterref_2 (Utilities|Array|Get(acopy) (Variables|Default|GetLightAttacks) (Variables|/Game/ThirdPerson/Blueprints/BP_ThirdPersonCharacter1.BP_ThirdPersonCharacter1_C|GetChainLightAttack _characterref_2)) 1.0 "None")
      (Variables|/Game/ThirdPerson/Blueprints/BP_ThirdPersonCharacter1.BP_ThirdPersonCharacter1_C|SetChainLightAttack (Variables|Default|GetCharacterRef) 3))
    (:3
      (Animation|PlayAnimMontage _characterref_2 (Utilities|Array|Get(acopy) (Variables|Default|GetLightAttacks) (Variables|/Game/ThirdPerson/Blueprints/BP_ThirdPersonCharacter1.BP_ThirdPersonCharacter1_C|GetChainLightAttack _characterref_2)) 1.0 "None")
      (Variables|/Game/ThirdPerson/Blueprints/BP_ThirdPersonCharacter1.BP_ThirdPersonCharacter1_C|SetChainLightAttack (Variables|Default|GetCharacterRef) 0))))

(event EventBeginPlay
  (bind _asbp_third_person_character (Utilities|Casting|CastToBP_ThirdPersonCharacter1 (Game|GetPlayerCharacter 0)))
  (Variables|Default|SetCharacterRef _asbp_third_person_character))