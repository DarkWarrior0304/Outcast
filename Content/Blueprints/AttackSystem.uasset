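; Player attack component for BP_ThirdPersonCharacter1, handling stamina-gated light, heavy and sprint sword attacks.
; Light and heavy inputs briefly turn the character toward control rotation and step through indexed montage combos, buffering presses until a combo-continue event.
; Stats component values set damage and combo play rate.
; A looping timer sphere-traces between sword points, damaging Enemy-tagged actors; StopHeavyAttack is an empty stub.
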(event Custom|Sword%20Sprint%20Attack
  ;[1 1 1] Sprint Attack
  ;;[1 1 1] Sword Attack
  (if (Variables|Default|GetisAttacking?)
    (Variables|Default|SetSave%20Sprint%20Attack true)
    (else
      (Variables|Default|SetisAttacking? true)
      (switch int (Variables|Default|GetSprint%20Attack%20Index)
        (:0
          (CallFunction|SprintAttack))
        (:1
          (CallFunction|SprintAttack2))))))

(event Custom|Continue%20Sprint%20Combo
  ;[1 1 1] Sprint Attack
  ;;[1 1 1] Combo Continue
  (if (Variables|Default|GetSave%20Sprint%20Attack)
    (Variables|Default|SetSave%20Sprint%20Attack false)
    (switch int (Variables|Default|GetSprint%20Attack%20Index)
      (:0
        (CallFunction|SprintAttack))
      (:1
        (CallFunction|SprintAttack2)))
    (else
      (CallFunction|StopSprintAttack))))

(event Custom|Sword%20Attack
  ;[1 1 1] Light Attack
  ;;[1 1 1] Sword Attack
  (if (Variables|Default|GetisAttacking?)
    (Variables|Default|SetsaveAttack true)
    (else
      (Variables|Default|SetisAttacking? true)
      (switch int (Variables|Default|GetAttack%20Index)
        (:0
          (CallFunction|Attack1))
        (:1
          (CallFunction|Attack2))
        (:2
          (CallFunction|Attack3))
        (:3
          (CallFunction|Attack4))))))

(event Custom|Sword%20Attck%20Combo
  ;[1 1 1] Light Attack
  ;;[1 1 1] Combo Continue
  (if (Variables|Default|GetsaveAttack)
    (Variables|Default|SetsaveAttack false)
    (switch int (Variables|Default|GetAttack%20Index)
      (:0
        (CallFunction|Attack1))
      (:1
        (CallFunction|Attack2))
      (:2
        (CallFunction|Attack3))
      (:3
        (CallFunction|Attack4)))
    (else
      (CallFunction|StopCombo))))

(event Custom|Stop%20Combo
  ;[1 1 1] Light Attack
  ;;[1 1 1] Stop Combo / Attack
  (Variables|Default|SetisAttacking? false)
  (Variables|Default|SetAttack%20Index 0)
  (Default|RegenStamina (Variables|Default|GetCharacter%20BP)))

(event Custom|Attack%201
  ;[1 1 1] Light Attack
  ;;[1 1 1] Attack 1
  (Utilities|FlowControl|DoOnce false :!label _label
    (:Completed
      (if (Variables|/Game/ThirdPerson/Blueprints/BP_ThirdPersonCharacter1.BP_ThirdPersonCharacter1_C|GetTarget%20Locked (Variables|Default|GetCharacter%20BP))
        (Default|FaceTarget (Variables|Default|GetCharacter%20BP)))
      (Utilities|FlowControl|Delay 0.1)
      (Animation|Montage|PlayMontage (Variables|Default|GetCharacter%20Mesh) "/Game/PlayerCharacter/Katana_Anims/Light_Attacks/Anim_Montages/ARPG_Samurai_Anim_UE_Attack_Combo1_Retargeted_Montage.ARPG_Samurai_Anim_UE_Attack_Combo1_Retargeted_Montage" (+ 1.0 (/ (.Value (Default|GetStatValue (Variables|/Game/RunesSystem/Blueprints/BP_RuneCharacter.BP_RuneCharacter_C|GetBP_StatsComponent (Variables|Default|GetCharacter%20BP)) "NewEnumerator6")) 1e+03))
        (:then
          (Default|StaminaDecrease (Variables|Default|GetCharacter%20BP) 5.0)
          (Variables|Default|SetAttack%20Index 1)
          (goto _label Reset))))))

(event Custom|Attack%202
  ;[1 1 1] Light Attack
  ;;[1 1 1] Attack 2
  (Utilities|FlowControl|DoOnce false :!label _label
    (:Completed
      (if (Variables|/Game/ThirdPerson/Blueprints/BP_ThirdPersonCharacter1.BP_ThirdPersonCharacter1_C|GetTarget%20Locked (Variables|Default|GetCharacter%20BP))
        (Default|FaceTarget (Variables|Default|GetCharacter%20BP)))
      (Utilities|FlowControl|Delay 0.1)
      (Animation|Montage|PlayMontage (Variables|Default|GetCharacter%20Mesh) "/Game/PlayerCharacter/Katana_Anims/Light_Attacks/Anim_Montages/ARPG_Samurai_Anim_UE_Attack_Combo2_Retargeted_Montage.ARPG_Samurai_Anim_UE_Attack_Combo2_Retargeted_Montage" (+ 1.0 (/ (.Value (Default|GetStatValue (Variables|/Game/RunesSystem/Blueprints/BP_RuneCharacter.BP_RuneCharacter_C|GetBP_StatsComponent (Variables|Default|GetCharacter%20BP)) "NewEnumerator6")) 1e+03))
        (:then
          (Default|StaminaDecrease (Variables|Default|GetCharacter%20BP) 5.0)
          (Variables|Default|SetAttack%20Index 2)
          (goto _label Reset))))))

(event Custom|Attack%203
  ;[1 1 1] Light Attack
  ;;[1 1 1] Attack 3
  (Utilities|FlowControl|DoOnce false :!label _label
    (:Completed
      (if (Variables|/Game/ThirdPerson/Blueprints/BP_ThirdPersonCharacter1.BP_ThirdPersonCharacter1_C|GetTarget%20Locked (Variables|Default|GetCharacter%20BP))
        (Default|FaceTarget (Variables|Default|GetCharacter%20BP)))
      (Utilities|FlowControl|Delay 0.1)
      (Animation|Montage|PlayMontage (Variables|Default|GetCharacter%20Mesh) "/Game/PlayerCharacter/Katana_Anims/Light_Attacks/Anim_Montages/ARPG_Samurai_Anim_UE_Attack_Combo3_Retargeted_Montage.ARPG_Samurai_Anim_UE_Attack_Combo3_Retargeted_Montage" (+ 1.0 (/ (.Value (Default|GetStatValue (Variables|/Game/RunesSystem/Blueprints/BP_RuneCharacter.BP_RuneCharacter_C|GetBP_StatsComponent (Variables|Default|GetCharacter%20BP)) "NewEnumerator6")) 1e+03))
        (:then
          (Default|StaminaDecrease (Variables|Default|GetCharacter%20BP) 5.0)
          (Variables|Default|SetAttack%20Index 3)
          (goto _label Reset))))))

(event Custom|Attack%204
  ;[1 1 1] Light Attack
  ;;[1 1 1] Attack 4
  (Utilities|FlowControl|DoOnce false :!label _label
    (:Completed
      (if (Variables|/Game/ThirdPerson/Blueprints/BP_ThirdPersonCharacter1.BP_ThirdPersonCharacter1_C|GetTarget%20Locked (Variables|Default|GetCharacter%20BP))
        (Default|FaceTarget (Variables|Default|GetCharacter%20BP)))
      (Utilities|FlowControl|Delay 0.1)
      (Animation|Montage|PlayMontage (Variables|Default|GetCharacter%20Mesh) "/Game/PlayerCharacter/Katana_Anims/Light_Attacks/Anim_Montages/ARPG_Samurai_Anim_UE_Attack_Combo4_Retargeted_Montage.ARPG_Samurai_Anim_UE_Attack_Combo4_Retargeted_Montage" (+ 1.0 (/ (.Value (Default|GetStatValue (Variables|/Game/RunesSystem/Blueprints/BP_RuneCharacter.BP_RuneCharacter_C|GetBP_StatsComponent (Variables|Default|GetCharacter%20BP)) "NewEnumerator6")) 1e+03))
        (:then
          (Default|StaminaDecrease (Variables|Default|GetCharacter%20BP) 5.0)
          (Variables|Default|SetAttack%20Index 0)
          (goto _label Reset))))))

(event Custom|Heavy%20Attack%20Combo
  ;[1 1 1] Heavy Attack
  ;;[1 1 1] Combo Continue
  (if (Variables|Default|GetSave%20Heavy%20Attack)
    (Variables|Default|SetSave%20Heavy%20Attack false)
    (switch int (Variables|Default|GetHeavy%20Attack%20Index)
      (:0
        (CallFunction|Heavy1))
      (:1
        (CallFunction|Heavy2)))
    (else
      (CallFunction|StopHeavyAttack))))

(event Custom|Stop%20Heavy%20Combo
  ;[1 1 1] Heavy Attack
  ;;[1 1 1] Stop Combo / Attack
  (Variables|Default|SetisAttacking? false)
  (Variables|Default|SetHeavy%20Attack%20Index 0)
  (Default|RegenStamina (Variables|Default|GetCharacter%20BP)))

(event Custom|Heavy%20Start
  ;[1 1 1] Heavy Attack
  ;;[1 1 1] Attack 1
  (Utilities|FlowControl|DoOnce false :!label _label
    (:Completed
      (Utilities|FlowControl|Delay 0.1)
      (Animation|Montage|PlayMontage (Variables|Default|GetCharacter%20Mesh) "/Game/PlayerCharacter/Katana_Anims/Heavy_Attacks/Anim_Montages/ARPG_Samurai_Anim_UE_Attack_Heavy1_Start_Retargeted_Montage.ARPG_Samurai_Anim_UE_Attack_Heavy1_Start_Retargeted_Montage"
        (:then
          (Variables|Default|SetHeavy%20Attack%20Index 1)
          (goto _label Reset))))))

(event Custom|Stop%20Sprint%20Attack
  ;[1 1 1] Sprint Attack
  ;;[1 1 1] Stop Combo / Attack
  (Variables|Default|SetisAttacking? false)
  (Variables|Default|SetSprint%20Attack%20Index 0)
  (Default|RegenStamina (Variables|Default|GetCharacter%20BP)))

(event Custom|Heavy%201
  ;[1 1 1] Heavy Attack
  ;;[1 1 1] Attack 2
  (Utilities|FlowControl|DoOnce false :!label _label
    (:Completed
      (Utilities|FlowControl|Delay 0.1)
      (Animation|Montage|PlayMontage (Variables|Default|GetCharacter%20Mesh) "/Game/PlayerCharacter/Katana_Anims/Heavy_Attacks/Anim_Montages/ARPG_Samurai_Anim_UE_Attack_Heavy1_Retargeted_Montage.ARPG_Samurai_Anim_UE_Attack_Heavy1_Retargeted_Montage" (+ 1.0 (/ (.Value (Default|GetStatValue (Variables|/Game/RunesSystem/Blueprints/BP_RuneCharacter.BP_RuneCharacter_C|GetBP_StatsComponent (Variables|Default|GetCharacter%20BP)) "NewEnumerator6")) 1e+03))
        (:then
          (Default|StaminaDecrease (Variables|Default|GetCharacter%20BP) 1e+01)
          (Variables|Default|SetHeavy%20Attack%20Index 1)
          (goto _label Reset))))))

(event Custom|Sprint%20Attack%202
  ;[1 1 1] Sprint Attack
  ;;[1 1 1] Attack 2
  (Utilities|FlowControl|DoOnce false :!label _label
    (:Completed
      (Utilities|FlowControl|Delay 0.1)
      (Animation|Montage|PlayMontage (Variables|Default|GetCharacter%20Mesh) "/Game/PlayerCharacter/Katana_Anims/Heavy_Attacks/Anim_Montages/ARPG_Samurai_Anim_UE_Attack_Heavy2_Retargeted_Montage.ARPG_Samurai_Anim_UE_Attack_Heavy2_Retargeted_Montage"
        (:then
          (Default|StaminaDecrease (Variables|Default|GetCharacter%20BP) 1e+01)
          (Variables|Default|SetSprint%20Attack%20Index 0)
          (goto _label Reset))))))

(event Custom|Heavy%202
  ;[1 1 1] Heavy Attack
  ;;[1 1 1] Attack 3
  (Utilities|FlowControl|DoOnce false :!label _label
    (:Completed
      (Utilities|FlowControl|Delay 0.1)
      (Animation|Montage|PlayMontage (Variables|Default|GetCharacter%20Mesh) "/Game/PlayerCharacter/Katana_Anims/Heavy_Attacks/Anim_Montages/ARPG_Samurai_Anim_UE_Attack_Heavy2_Retargeted_Montage.ARPG_Samurai_Anim_UE_Attack_Heavy2_Retargeted_Montage" (+ 1.0 (/ (.Value (Default|GetStatValue (Variables|/Game/RunesSystem/Blueprints/BP_RuneCharacter.BP_RuneCharacter_C|GetBP_StatsComponent (Variables|Default|GetCharacter%20BP)) "NewEnumerator6")) 1e+03))
        (:then
          (Default|StaminaDecrease (Variables|Default|GetCharacter%20BP) 1e+01)
          (Variables|Default|SetHeavy%20Attack%20Index 0)
          (goto _label Reset))))))

(event Custom|Sword%20Heavy%20Attack
  ;[1 1 1] Heavy Attack
  ;;[1 1 1] Sword Attack
  (if (Variables|Default|GetisAttacking?)
    (Variables|Default|SetSave%20Heavy%20Attack true)
    (else
      (Variables|Default|SetisAttacking? true)
      (switch int (Variables|Default|GetHeavy%20Attack%20Index)
        (:0
          (CallFunction|Heavy1))
        (:1
          (CallFunction|Heavy2))))))

(event Custom|Sprint%20Attack
  ;[1 1 1] Sprint Attack
  ;;[1 1 1] Attack 1
  (Utilities|FlowControl|DoOnce false :!label _label
    (:Completed
      (Utilities|FlowControl|Delay 0.1)
      (Animation|Montage|PlayMontage (Variables|Default|GetCharacter%20Mesh) "/Game/PlayerCharacter/Katana_Anims/Sprint_Attacks/Montages/ARPG_Samurai_Anim_UE_Attack_Sprint_Retargeted_Montage.ARPG_Samurai_Anim_UE_Attack_Sprint_Retargeted_Montage"
        (:then
          (Variables|Default|SetCan%20Sprint%20Attack false)
          (Default|StaminaDecrease (Variables|Default|GetCharacter%20BP) 5.0)
          (Variables|Default|SetSprint%20Attack%20Index 1)
          (goto _label Reset))
        (:OnCompleted
          (Variables|Default|SetCan%20Sprint%20Attack true))))))

(event Custom|Start%20Sword%20Trace
  ;[1 1 1] Sword Trace
  (bind _returnvalue (Utilities|Time|SetTimerbyEvent (delegate Custom|Sword%20Trace%20Loop) 0.001 true))
  (Variables|Default|SetSwordTraceLoop _returnvalue))

(event Custom|Sword%20Trace%20Loop
  ;[1 1 1] Sword Trace
  (bind (_outhit _returnvalue) (Collision|SphereTraceByChannel (Transformation|GetWorldLocation (Variables|/Game/ThirdPerson/Blueprints/BP_ThirdPersonCharacter1.BP_ThirdPersonCharacter1_C|GetSword%20Top%20Point (Variables|Default|GetCharacter%20BP))) (Transformation|GetWorldLocation (Variables|/Game/ThirdPerson/Blueprints/BP_ThirdPersonCharacter1.BP_ThirdPersonCharacter1_C|GetSword%20Bottom%20Point (Variables|Default|GetCharacter%20BP))) 12.0 "TraceTypeQuery1" false 0 "None" true "(R=1.000000,G=0.000000,B=0.000000,A=1.000000)" "(R=0.000000,G=1.000000,B=0.000000,A=1.000000)" 0.1))
  (if _returnvalue
    (if (Actor|ActorHasTag (.HitActor (Collision|BreakHitResult _outhit)) "Enemy")
      (Utilities|FlowControl|DoOnce false :!label _label
        (:Completed
          (Game|Damage|ApplyDamage (.HitActor (Collision|BreakHitResult _outhit)) (Variables|Default|GetDamage) 0 0)
          (Utilities|FlowControl|Delay 0.5)
          (goto _label Reset))))))

(event Custom|Stop%20Sword%20Trace
  ;[1 1 1] Sword Trace
  (Utilities|Time|ClearandInvalidateTimerbyHandle (Variables|Default|GetSwordTraceLoop)))

(event Input|EnhancedActionEvents|EnhancedInputActionIA_LightAttack
  (params (ActionValue :type Boolean) (ElapsedSeconds :type Float%20%28double-precision%29) (TriggeredSeconds :type Float%20%28double-precision%29) (InputAction :type Input%20Action%20Object%20Reference :default "/Game/ThirdPerson/Input/Actions/IA_LightAttack.IA_LightAttack"))
  ;[1 1 1] Stamina Check
  (:Triggered
    (if (< (Variables|/Game/ThirdPerson/Blueprints/BP_ThirdPersonCharacter1.BP_ThirdPersonCharacter1_C|GetStamina (Variables|Default|GetCharacter%20BP)) 5.0)
      (Variables|Default|SetcanAttack? false)
      (else
        (Variables|Default|SetcanAttack? true)))))

(event Input|EnhancedActionEvents|EnhancedInputActionIA_HeavyAttack
  (params (ActionValue :type Boolean) (ElapsedSeconds :type Float%20%28double-precision%29) (TriggeredSeconds :type Float%20%28double-precision%29) (InputAction :type Input%20Action%20Object%20Reference :default "/Game/ThirdPerson/Input/Actions/IA_HeavyAttack.IA_HeavyAttack"))
  ;[1 1 1] Stamina Check
  (:Triggered
    (if (< (Variables|/Game/ThirdPerson/Blueprints/BP_ThirdPersonCharacter1.BP_ThirdPersonCharacter1_C|GetStamina (Variables|Default|GetCharacter%20BP)) 1e+01)
      (Variables|Default|SetCan%20Heavy%20Attack false)
      (else
        (Variables|Default|SetCan%20Heavy%20Attack true)))))

(event Input|EnhancedActionEvents|EnhancedInputActionIA_SprintAttack
  (params (ActionValue :type Boolean) (ElapsedSeconds :type Float%20%28double-precision%29) (TriggeredSeconds :type Float%20%28double-precision%29) (InputAction :type Input%20Action%20Object%20Reference :default "/Game/ThirdPerson/Input/Actions/IA_SprintAttack.IA_SprintAttack"))
  ;[1 1 1] Stamina Check
  (:Triggered
    (if (< (Variables|/Game/ThirdPerson/Blueprints/BP_ThirdPersonCharacter1.BP_ThirdPersonCharacter1_C|GetStamina (Variables|Default|GetCharacter%20BP)) 5.0)
      (Variables|Default|SetCan%20Sprint%20Attack false)
      (else
        (Variables|Default|SetCan%20Sprint%20Attack true)))))

(event Input|EnhancedActionEvents|EnhancedInputActionIA_LightAttack
  (params (ActionValue :type Boolean) (ElapsedSeconds :type Float%20%28double-precision%29) (TriggeredSeconds :type Float%20%28double-precision%29) (InputAction :type Input%20Action%20Object%20Reference :default "/Game/ThirdPerson/Input/Actions/IA_LightAttack.IA_LightAttack"))
  ;[1 1 1] Light Attack
  ;;[1 1 1] Attack Input
  (:Triggered
    (if (Variables|Default|GetcanAttack?)
      (CallFunction|SwordAttack)
      (Variables|Default|SetOrient%20Attack true)
      (Utilities|FlowControl|Delay 0.3)
      (Variables|Default|SetOrient%20Attack false)
      (Variables|Default|SetDamage (.Value (Default|GetStatValue (Variables|/Game/RunesSystem/Blueprints/BP_RuneCharacter.BP_RuneCharacter_C|GetBP_StatsComponent (Variables|Default|GetCharacter%20BP)) "NewEnumerator2"))))))

(event Input|EnhancedActionEvents|EnhancedInputActionIA_HeavyAttack
  (params (ActionValue :type Boolean) (ElapsedSeconds :type Float%20%28double-precision%29) (TriggeredSeconds :type Float%20%28double-precision%29) (InputAction :type Input%20Action%20Object%20Reference :default "/Game/ThirdPerson/Input/Actions/IA_HeavyAttack.IA_HeavyAttack"))
  ;[1 1 1] Heavy Attack
  ;;[1 1 1] Attack Input
  (:Triggered
    (if (Variables|Default|GetCan%20Heavy%20Attack)
      (CallFunction|SwordHeavyAttack)
      (Variables|Default|SetOrient%20Attack true)
      (Utilities|FlowControl|Delay 0.3)
      (Variables|Default|SetOrient%20Attack false)
      (Variables|Default|SetDamage (* (.Value (Default|GetStatValue (Variables|/Game/RunesSystem/Blueprints/BP_RuneCharacter.BP_RuneCharacter_C|GetBP_StatsComponent (Variables|Default|GetCharacter%20BP)) "NewEnumerator2")) 1.5)))))

(event Input|EnhancedActionEvents|EnhancedInputActionIA_SprintAttack
  (params (ActionValue :type Boolean) (ElapsedSeconds :type Float%20%28double-precision%29) (TriggeredSeconds :type Float%20%28double-precision%29) (InputAction :type Input%20Action%20Object%20Reference :default "/Game/ThirdPerson/Input/Actions/IA_SprintAttack.IA_SprintAttack"))
  ;[1 1 1] Sprint Attack
  ;;[1 1 1] Attack Input
  (:Triggered
    (Utilities|FlowControl|DoOnce false :!label _label
      (:Completed
        (if (Variables|Default|GetCan%20Sprint%20Attack)
          (if (not (Variables|Default|GetisAttacking?))
            (Variables|Default|SetisAttacking? true)
            (Variables|Default|SetCan%20Sprint%20Attack false)
            (Animation|Montage|PlayMontage (Variables|Default|GetCharacter%20Mesh) "/Game/PlayerCharacter/Katana_Anims/Sprint_Attacks/Montages/ARPG_Samurai_Anim_UE_Attack_Sprint_Retargeted_Montage.ARPG_Samurai_Anim_UE_Attack_Sprint_Retargeted_Montage"
              (:OnCompleted
                _)
              (:OnInterrupted
                _))
            (Variables|Default|SetCan%20Sprint%20Attack true)
            (Variables|Default|SetisAttacking? false)
            (Default|StaminaDecrease (Variables|Default|GetCharacter%20BP) 5.0)
            (Variables|Default|SetDamage (* (.Value (Default|GetStatValue (Variables|/Game/RunesSystem/Blueprints/BP_RuneCharacter.BP_RuneCharacter_C|GetBP_StatsComponent (Variables|Default|GetCharacter%20BP)) "NewEnumerator2")) 1.2))
            (Utilities|FlowControl|Delay 0.2)
            (goto _label Reset)))))))

(event EventBeginPlay
  ;[1 1 1] Cast to Character
  (bind _asbp_third_person_character_1 (Utilities|Casting|CastToBP_ThirdPersonCharacter1 (Components|GetOwner)))
  (Variables|Default|SetCharacter%20BP _asbp_third_person_character_1)
  (Variables|Default|SetCharacter%20Mesh (Variables|/Script/Engine.Character|GetMesh _asbp_third_person_character_1)))

(event EventTick
  (params (DeltaSeconds :type Float%20%28single-precision%29))
  (bind _character_bp (Variables|Default|GetCharacter%20BP))
  (bind _returnvalue (Transformation|GetActorRotation _character_bp))
  (bind (_roll _pitch) (Math|Rotator|BreakRotator _returnvalue))
  ;[1 1 1] Attack Orientation
  (if (Variables|Default|GetOrient%20Attack)
    (Transformation|SetActorRotation _character_bp (Math|Rotator|MakeRotator _roll _pitch (.yaw (Math|Interpolation|RInterpTo _returnvalue (Pawn|GetControlRotation _character_bp :!class /Script/Engine.Pawn) DeltaSeconds 1e+01))))))

(fn StopHeavyAttack)