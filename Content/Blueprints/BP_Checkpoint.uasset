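; Checkpoint actor, styled as a wishing well, that records itself as the player's last checkpoint when used.
; Its Trigger overlap sets or clears CheckpointRef on BP_ThirdPersonCharacter1.
; EnterCheckpointMenu opens WishingWellMenu with UI-only input and a cursor, then saves the checkpoint on the player character; LeaveCheckpointMenu restores game input.
; An InteractTooltip is created at BeginPlay but never displayed, as that logic and the mapping-context switching are disconnected.
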(event OnComponentBeginOverlap(Trigger)
  (params (OverlappedComponent :type Primitive%20Component%20Object%20Reference) (OtherActor :type Actor%20Object%20Reference) (OtherComp :type Primitive%20Component%20Object%20Reference) (OtherBodyIndex :type Integer) (bFromSweep :type Boolean) (SweepResult :type Hit%20Result%20Structure%20%28by%20ref%29))
  (Development|PrintString "Checkpoint")
  (bind _ascharacter (Utilities|Casting|CastToCharacter OtherActor))
  (bind _asbp_third_person_character_1 (Utilities|Casting|CastToBP_ThirdPersonCharacter1 _ascharacter))
  (Variables|/Game/ThirdPerson/Blueprints/BP_ThirdPersonCharacter1.BP_ThirdPersonCharacter1_C|SetCheckpointRef _asbp_third_person_character_1 self))

(event OnComponentEndOverlap(Trigger)
  (params (OverlappedComponent :type Primitive%20Component%20Object%20Reference) (OtherActor :type Actor%20Object%20Reference) (OtherComp :type Primitive%20Component%20Object%20Reference) (OtherBodyIndex :type Integer))
  (bind _ascharacter (Utilities|Casting|CastToCharacter OtherActor))
  (bind _asbp_third_person_character_1 (Utilities|Casting|CastToBP_ThirdPersonCharacter1 _ascharacter))
  (Variables|/Game/ThirdPerson/Blueprints/BP_ThirdPersonCharacter1.BP_ThirdPersonCharacter1_C|SetCheckpointRef _asbp_third_person_character_1 0))

(event Custom|Set%20Checkpoint
  (bind _asbp_third_person_character_1 (Utilities|Casting|CastToBP_ThirdPersonCharacter1 (Game|GetPlayerCharacter 0)))
  (Variables|/Game/ThirdPerson/Blueprints/BP_ThirdPersonCharacter1.BP_ThirdPersonCharacter1_C|SetLast%20Checkpoint _asbp_third_person_character_1 self))

(event Custom|Use%20Well
  (bind _returnvalue (Game|GetPlayerController 0))
  (Widget|RemovefromParent (Variables|Default|GetText%20Ref))
  (bind _returnvalue_2 (UserInterface|CreateWidget "/Game/UI/WishingWellMenu.WishingWellMenu_C"))
  (bind _output_get (Variables|Default|SetMenuRef _returnvalue_2))
  (UserInterface|Viewport|AddtoViewport _output_get 0)
  (Input|SetInputModeUIOnly _returnvalue (Variables|Default|GetMenuRef) "DoNotLock" false)
  (Variables|/Script/Engine.PlayerController|SetbShowMouseCursor _returnvalue true)
  (CallFunction|SetCheckpoint))

(event EventBeginPlay
  (bind _returnvalue (UserInterface|CreateWidget "/Game/UI/InteractTooltip.InteractTooltip_C"))
  (Variables|Default|SetText%20Ref _returnvalue))

(event Collision|EventActorBeginOverlap
  (params (OtherActor :type Actor%20Object%20Reference)))

(event EventTick
  (params (DeltaSeconds :type Float%20%28single-precision%29)))

(event EventLeaveCheckpointMenu
  (bind _returnvalue (Game|GetPlayerController 0))
  (Widget|RemovefromParent (Variables|Default|GetMenuRef))
  (Input|SetInputModeGameOnly _returnvalue false)
  (Variables|/Script/Engine.PlayerController|SetbShowMouseCursor _returnvalue false))

(event EventEnterCheckpointMenu
  (CallFunction|UseWell))

(event EventSetCheckpoint
  (CallFunction|SetCheckpoint))

(fn ConstructionScript)