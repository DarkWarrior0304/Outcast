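; Sword-wielding AI enemy with a camera-facing health bar, a lock-on reticle, and death on zero health that notifies the player character.
; Attack, apparently driven by a behavior tree, starts a montage combo alternating two attacks, with buffered continuation; Attack3 and Attack4 are unwired.
; A looping-timer sphere trace along the blade damages Player-tagged actors, throttled by a delayed DoOnce.
; Tick updates the health bar's rotation and fill.
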(event Custom|Sword%20Attack%20Combo%20Call%20From%20BT
  ;[1 1 1] Light Attack
  ;;[1 1 1] Attack Input
  (if (Variables|Default|GetcanAttack?)
    (CallFunction|SwordAttack)
    (Utilities|FlowControl|Delay 0.3)
    (Variables|Default|SetDamage 45.0)))

(event Custom|Sword%20Attack
  ;[1 1 1] Light Attack
  ;;[1 1 1] Sword Attack
  (if (Variables|Default|GetisAttacking?)
    (Variables|Default|SetsaveAttack true)
    (else
      (Variables|Default|SetisAttacking? true)
      (switch int (Variables|Default|GetAttack%20Index)
        (:0
          (CallFunction|Attack1))
        (:1
          (CallFunction|Attack2))))))

(event Custom|Sword%20Attck%20Combo
  ;[1 1 1] Light Attack
  ;;[1 1 1] Combo Continue
  (if (Variables|Default|GetsaveAttack)
    (Variables|Default|SetsaveAttack false)
    (switch int (Variables|Default|GetAttack%20Index)
      (:0
        (CallFunction|Attack1))
      (:1
        (CallFunction|Attack2)))
    (else
      (CallFunction|StopCombo))))

(event Custom|Stop%20Combo
  ;[1 1 1] Light Attack
  ;;[1 1 1] Stop Combo / Attack
  (Variables|Default|SetisAttacking? false)
  (Variables|Default|SetAttack%20Index 0))

(event Custom|Attack%201
  ;[1 1 1] Light Attack
  ;;[1 1 1] Attack 1
  (Utilities|FlowControl|DoOnce false :!label _label
    (:Completed
      (Utilities|FlowControl|Delay 0.1)
      (Animation|Montage|PlayMontage (Variables|Character|GetMesh) "/Game/AI_Standard/Animations/Montage_SwordCombo.Montage_SwordCombo"
        (:then
          (Variables|Default|SetAttack%20Index 1)
          (goto _label Reset))))))

(event Custom|Attack%202
  ;[1 1 1] Light Attack
  ;;[1 1 1] Attack 2
  (Utilities|FlowControl|DoOnce false :!label _label
    (:Completed
      (Utilities|FlowControl|Delay 0.1)
      (Animation|Montage|PlayMontage (Variables|Character|GetMesh) "/Game/AI_Standard/Animations/Montage_SwordCombo.Montage_SwordCombo"
        (:then
          (Variables|Default|SetAttack%20Index 0)
          (goto _label Reset))))))

(event Custom|Attack%203
  ;[1 1 1] Light Attack
  ;;[1 1 1] Attack 3
  (Utilities|FlowControl|DoOnce false :!label _label
    (:Completed
      (Utilities|FlowControl|Delay 0.1)
      (Animation|Montage|PlayMontage (Variables|Character|GetMesh) "/Game/Enemies/Animations/Boss/Attack/Montages/ARPG_Samurai_Anim_UE_Attack_Combo3_Retargeted_Montage.ARPG_Samurai_Anim_UE_Attack_Combo3_Retargeted_Montage"
        (:then
          (Variables|Default|SetAttack%20Index 3)
          (goto _label Reset))))))

(event Custom|Attack%204
  ;[1 1 1] Light Attack
  ;;[1 1 1] Attack 4
  (Utilities|FlowControl|DoOnce false :!label _label
    (:Completed
      (Utilities|FlowControl|Delay 0.1)
      (Animation|Montage|PlayMontage (Variables|Character|GetMesh) "/Game/Enemies/Animations/Boss/Attack/Montages/ARPG_Samurai_Anim_UE_Attack_Combo4_Retargeted_Montage.ARPG_Samurai_Anim_UE_Attack_Combo4_Retargeted_Montage"
        (:then
          (Variables|Default|SetAttack%20Index 0)
          (goto _label Reset))))))

(event Custom|Start%20Sword%20Trace
  ;[1 1 1] Sword Trace
  (bind _returnvalue (Utilities|Time|SetTimerbyEvent (delegate Custom|Sword%20Trace%20Loop) 0.001 true))
  (Variables|Default|SetSwordTraceLoop _returnvalue))

(event Custom|Sword%20Trace%20Loop
  ;[1 1 1] Sword Trace
  (bind (_outhit _returnvalue) (Collision|SphereTraceByChannel (Transformation|GetWorldLocation (Variables|Default|GetSword%20Top%20Point)) (Transformation|GetWorldLocation (Variables|Default|GetSword%20Bottom%20Point)) 12.0 "TraceTypeQuery1" false 0 "None" true "(R=1.000000,G=0.000000,B=0.000000,A=1.000000)" "(R=0.000000,G=1.000000,B=0.000000,A=1.000000)" 0.1))
  (if _returnvalue
    (if (Actor|ActorHasTag (.HitActor (Collision|BreakHitResult _outhit)) "Player")
      (Utilities|FlowControl|DoOnce false :!label _label
        (:Completed
          (Game|Damage|ApplyDamage (.HitActor (Collision|BreakHitResult _outhit)) (Variables|Default|GetDamage) 0 0)
          (Utilities|FlowControl|Delay 0.5)
          (goto _label Reset))))))

(event Custom|Stop%20Sword%20Trace
  ;[1 1 1] Sword Trace
  (Utilities|Time|ClearandInvalidateTimerbyHandle (Variables|Default|GetSwordTraceLoop)))

(event EventBeginPlay
  (Utilities|FlowControl|Sequence
    (:then_0
      (Utilities|Casting|CastToEnemy_Health (UserInterface|GetWidget (Variables|Default|GetHealth%20Bar))))
    (:then_1
      (Variables|Default|SetEnemy%20Health (Variables|Default|GetEnemy%20Max%20Health)))))

(event Collision|EventActorBeginOverlap
  (params (OtherActor :type Actor%20Object%20Reference)))

(event EventTick
  (params (DeltaSeconds :type Float%20%28single-precision%29))
  (Utilities|FlowControl|Sequence
    (:then_0
      (Transformation|SetWorldRotation (Variables|Default|GetHealth%20Bar) (Math|Rotator|FindLookatRotation (Transformation|GetWorldLocation (Variables|Default|GetHealth%20Bar)) (Transformation|GetWorldLocation (Variables|/Script/Engine.PlayerCameraManager|GetTransformComponent (Game|GetPlayerCameraManager 0)))) false false))
    (:then_1
      (CallFunction|UpdateHealthBar))))

(event EventUntargeted
  (Rendering|SetVisibility (Variables|Default|GetLock%20On%20Reticle) false false))

(event EventTargeted
  (Rendering|SetVisibility (Variables|Default|GetLock%20On%20Reticle) true false))

(event Game|Damage|EventAnyDamage
  (params (Damage :type Float%20%28single-precision%29) (DamageType :type Damage%20Type%20Object%20Reference) (InstigatedBy :type Controller%20Object%20Reference) (DamageCauser :type Actor%20Object%20Reference))
  (Rendering|SetVisibility (Variables|Default|GetHealth%20Bar) true false)
  (bind _output_get (Variables|Default|SetEnemy%20Health (- (Variables|Default|GetEnemy%20Health) Damage)))
  (if (<= _output_get 0.0)
    (Actor|DestroyActor)
    (bind _returnvalue (Actor|GetActorOfClass "/Game/ThirdPerson/Blueprints/BP_ThirdPersonCharacter1.BP_ThirdPersonCharacter1_C"))
    (Class|BPIEnemyDeath|EnemyDeath(Message) _returnvalue)))

(fn ConstructionScript)

(fn NewFunction0)

(fn UpdateHealthBar
  (bind _asenemy_health (Utilities|Casting|CastToEnemy_Health (UserInterface|GetUserWidgetObject (Variables|Default|GetHealth%20Bar))))
  (Progress|SetPercent (Variables|/Game/UI/Enemy_Health.Enemy_Health_C|GetHealthBar _asenemy_health) (/ (Variables|Default|GetEnemy%20Health) (Variables|Default|GetEnemy%20Max%20Health)))
  (return))

(fn Attack
  (CallFunction|SwordAttackComboCallfromBT)
  (return 0.4))