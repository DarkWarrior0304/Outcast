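; BP_DummyEnemy is a damageable dummy enemy that can be targeted by lock-on.
; Targeted and Untargeted toggle its reticle, while Tick rotates the health bar widget toward the camera and refreshes its fill.
; Damage reveals the bar and lowers health; at zero it hides both indicators, notifies BP_ThirdPersonCharacter1, plays a death animation and destroys itself after a delay.
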(event EventBeginPlay
  (Utilities|FlowControl|Sequence
    (:then_0
      (Utilities|Casting|CastToEnemy_Health (UserInterface|GetWidget (Variables|Default|GetHealth%20Bar))))
    (:then_1
      (Variables|Default|SetEnemy%20Health (Variables|Default|GetEnemy%20Max%20Health)))))

(event Collision|EventActorBeginOverlap
  (params (OtherActor :type Actor%20Object%20Reference)))

(event EventTick
  (params (DeltaSeconds :type Float%20%28single-precision%29))
  (Utilities|FlowControl|Sequence
    (:then_0
      (Transformation|SetWorldRotation (Variables|Default|GetHealth%20Bar) (Math|Rotator|FindLookatRotation (Transformation|GetWorldLocation (Variables|Default|GetHealth%20Bar)) (Transformation|GetWorldLocation (Variables|/Script/Engine.PlayerCameraManager|GetTransformComponent (Game|GetPlayerCameraManager 0)))) false false))
    (:then_1
      (CallFunction|UpdateHealthBar))))

(event EventUntargeted
  (Rendering|SetVisibility (Variables|Default|GetLock%20On%20Reticle) false false))

(event EventTargeted
  (Rendering|SetVisibility (Variables|Default|GetLock%20On%20Reticle) true false))

(event Game|Damage|EventAnyDamage
  (params (Damage :type Float%20%28single-precision%29) (DamageType :type Damage%20Type%20Object%20Reference) (InstigatedBy :type Controller%20Object%20Reference) (DamageCauser :type Actor%20Object%20Reference))
  (Rendering|SetVisibility (Variables|Default|GetHealth%20Bar) true false)
  (bind _output_get (Variables|Default|SetEnemy%20Health (- (Variables|Default|GetEnemy%20Health) Damage)))
  (if (<= _output_get 0.0)
    (Rendering|SetVisibility (Variables|Default|GetLock%20On%20Reticle) false false)
    (Rendering|SetVisibility (Variables|Default|GetHealth%20Bar) false false)
    (bind _returnvalue (Actor|GetActorOfClass "/Game/ThirdPerson/Blueprints/BP_ThirdPersonCharacter1.BP_ThirdPersonCharacter1_C"))
    (Class|BPIEnemyDeath|EnemyDeath(Message) _returnvalue)
    (Components|Animation|PlayAnimation (Variables|Character|GetMesh) "/Game/Enemies/Animations/Boss/ARPG_Samurai_Anim_UE_Death2_Retargeted.ARPG_Samurai_Anim_UE_Death2_Retargeted" false)
    (Utilities|FlowControl|Delay 3.0)
    (Actor|DestroyActor)))

(fn ConstructionScript)

(fn NewFunction0)

(fn UpdateHealthBar
  (bind _asenemy_health (Utilities|Casting|CastToEnemy_Health (UserInterface|GetUserWidgetObject (Variables|Default|GetHealth%20Bar))))
  (Progress|SetPercent (Variables|/Game/UI/Enemy_Health.Enemy_Health_C|GetHealthBar _asenemy_health) (/ (Variables|Default|GetEnemy%20Health) (Variables|Default|GetEnemy%20Max%20Health)))
  (return))